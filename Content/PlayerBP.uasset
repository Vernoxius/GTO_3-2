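; Player Blueprint that slides the actor side to side along the world Y axis within fixed bounds.
; Each Tick reads the Z component of a vector axis input, ignoring a central dead zone; positive values move toward -Y and negative toward +Y.
; Movement is a fixed per-frame SetActorLocation step without sweep or delta-time scaling, so speed depends on frame rate.
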(event EventBeginPlay)

(event Collision|EventActorBeginOverlap
  (params (OtherActor :type Actor%20Object%20Reference)))

(event EventTick
  (params (DeltaSeconds :type Float%20%28single-precision%29))
  (bind _returnvalue (Transformation|GetActorLocation))
  (bind _returnvalue_2 (Transformation|GetActorLocation))
  (bind (_x _y _z) (Math|Vector|BreakVector _returnvalue))
  (bind (_x_2 _y_2 _z_2) (Math|Vector|BreakVector _returnvalue_2))
  (bind _output_get (Variables|Default|SetZValue (.Z (Math|Vector|BreakVector (Class|Actor|GetInputVectorAxisValue)))))
  (Math|Float|CompareFloat _output_get 0.4
    (:>
      (Math|Float|CompareFloat _y_2 -4.9e+02
        (:>
          (Transformation|SetActorLocation (Math|Vector|MakeVector _x_2 (- _y_2 5.0) _z_2) false false))))
    (:<
      (Math|Float|CompareFloat _output_get -0.4
        (:<
          (Math|Float|CompareFloat _y 4.9e+02
            (:<
              (Transformation|SetActorLocation (Math|Vector|MakeVector _x (+ 5.0 _y) _z) false false))))))))

(fn ConstructionScript)